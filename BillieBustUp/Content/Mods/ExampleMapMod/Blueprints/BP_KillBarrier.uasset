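; BP_KillBarrier is a trigger volume that kills the BP_BillieV2 character on contact.
; When an overlapping actor implements BPI_HitInterface and casts to BP_BillieV2, it lowers CurrentHealth below the damage it then deals through HitBIMessage, with invincibility suppressed.
; It then creates the DeathMenu widget itself, shows the mouse cursor and enables input on the barrier actor for the first player controller.
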(event `self.Box.OnComponentBeginOverlap`
  (params (OverlappedComponent :type "PrimitiveComponent Object Reference") (OtherActor :type "Actor Object Reference") (OtherComp :type "PrimitiveComponent Object Reference") (OtherBodyIndex :type Integer) (bFromSweep :type Boolean) (SweepResult :type "HitResult Structure (by ref)"))
  (bind _returnvalue (`GameplayStatics.GetPlayerController` 0))
  (if (`KismetSystemLibrary.DoesImplementInterface` OtherActor "/Game/Blueprints/Interfaces/BPI_HitInterface.BPI_HitInterface_C")
    (bind _asbp_billie_v2 (cast `/Game/Blueprints/Characters/BP_BillieV2` OtherActor))
    (set `/Game/Blueprints/Characters/BP_BillieV2.Current_Health` 12.5 _asbp_billie_v2)
    (message `/Game/Blueprints/Interfaces/BPI_HitInterface.Hit_BI` OtherActor 25 false false true 0 null false false false)
    (bind _returnvalue_2 (`|CreateWidget` "/Game/Mods/ExampleMapMod/UI/DeathMenu.DeathMenu_C" (`GameplayStatics.GetPlayerController` 0)))
    (`UserWidget.AddToViewport` _returnvalue_2 0)
    (set `PlayerController.bShowMouseCursor` true _returnvalue)
    (`self.EnableInput` _returnvalue)))

(fn `UserConstructionScript`)