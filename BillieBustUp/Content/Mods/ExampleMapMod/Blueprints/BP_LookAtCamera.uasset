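; BP_LookAtCamera is an example map mod Blueprint that keeps its SceneComponent turned toward the player's Billie pawn.
; Shortly after BeginPlay, a brief delay precedes casting player pawn 0 to BP_BillieV2 and caching it.
; Each Tick, while that reference is valid, it sets the component's world rotation with FindLookAtRotation, aiming at the pawn's actor location rather than a camera.
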(event `self.ReceiveBeginPlay`
  (`KismetSystemLibrary.Delay` 0.01)
  (bind _asbp_billie_v2 (cast `/Game/Blueprints/Characters/BP_BillieV2` (`GameplayStatics.GetPlayerPawn` 0)))
  (set `self.Billie` _asbp_billie_v2))

(event `self.ReceiveTick`
  (params (DeltaSeconds :type "Float (single-precision)"))
  (bind _billie (`self.Billie`))
  (`/Engine/EditorBlueprintResources/StandardMacros.IsValid` _billie
    (:`Is Valid`
      (`SceneComponent.K2_SetWorldRotation` (`self.SceneComponent`) (`KismetMathLibrary.FindLookAtRotation` (`SceneComponent.K2_GetComponentLocation` (`self.SceneComponent`)) (`self.K2_GetActorLocation` _billie)) false false))))

(fn `UserConstructionScript`)