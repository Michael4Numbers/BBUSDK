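; Trigger actor in the example map mod that turns the main camera when BP_BillieV2 enters its box.
; The overlap plays the RotateCamera timeline, which blends player 0's control rotation toward a target along the shortest path.
; IsRotationPlayerBased selects the target: Billie's mesh rotation or the actor's Arrow component.
; Each update lerps from the current control rotation rather than a cached start.
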(event `self.Box.OnComponentBeginOverlap`
  (params (OverlappedComponent :type "PrimitiveComponent Object Reference") (OtherActor :type "Actor Object Reference") (OtherComp :type "PrimitiveComponent Object Reference") (OtherBodyIndex :type Integer) (bFromSweep :type Boolean) (SweepResult :type "HitResult Structure (by ref)"))
  (bind _returnvalue (`GameplayStatics.GetPlayerController` 0))
  (bind _returnvalue_2 (`Controller.GetControlRotation` _returnvalue))
  (bind _asbp_billie_v2 (cast `/Game/Blueprints/Characters/BP_BillieV2` OtherActor))
  (set `self.Forward` (`Character.Mesh` _asbp_billie_v2))
  (bind (_direction _rotatetrack) (`Timeline|RotateCamera` :!via `PlayFromStart`)
    (:`Update`
      (if (`self.isRotationPlayerBased`)
        (`Controller.SetControlRotation` _returnvalue (`KismetMathLibrary.RLerp` _returnvalue_2 (`SceneComponent.K2_GetComponentRotation` (`self.Forward`)) _rotatetrack true))
        (else
          (`Controller.SetControlRotation` _returnvalue (`KismetMathLibrary.RLerp` _returnvalue_2 (`SceneComponent.K2_GetComponentRotation` (`self.Arrow`)) _rotatetrack true)))))))

(fn `UserConstructionScript`)