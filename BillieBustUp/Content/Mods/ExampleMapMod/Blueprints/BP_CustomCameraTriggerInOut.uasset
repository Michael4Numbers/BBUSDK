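; Trigger volume for the example map mod that switches the player's view to a custom camera while BP_BillieV2 is inside it.
; Box overlap begin blends player controller 0's view target to the assigned Camera, and overlap end blends it back to the player character.
; Both transitions share the same blend time, function and exponent variables.
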(event `self.Box.OnComponentBeginOverlap`
  (params (OverlappedComponent :type "PrimitiveComponent Object Reference") (OtherActor :type "Actor Object Reference") (OtherComp :type "PrimitiveComponent Object Reference") (OtherBodyIndex :type Integer) (bFromSweep :type Boolean) (SweepResult :type "HitResult Structure (by ref)"))
  (cast `/Game/Blueprints/Characters/BP_BillieV2` OtherActor)
  (`PlayerController.SetViewTargetWithBlend` (`GameplayStatics.GetPlayerController` 0) (`self.Camera`) (`self.BlendTime`) (`self.BlendFunc`) (`self.BlendExp`) false))

(event `self.Box.OnComponentEndOverlap`
  (params (OverlappedComponent :type "PrimitiveComponent Object Reference") (OtherActor :type "Actor Object Reference") (OtherComp :type "PrimitiveComponent Object Reference") (OtherBodyIndex :type Integer))
  (cast `/Game/Blueprints/Characters/BP_BillieV2` OtherActor)
  (`PlayerController.SetViewTargetWithBlend` (`GameplayStatics.GetPlayerController` 0) (`GameplayStatics.GetPlayerCharacter` 0) (`self.BlendTime`) (`self.BlendFunc`) (`self.BlendExp`) false))

(fn `UserConstructionScript`)