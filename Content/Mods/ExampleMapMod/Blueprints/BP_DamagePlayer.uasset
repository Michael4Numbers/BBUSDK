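; BP_DamagePlayer is a damage volume that hurts actors overlapping its Box.
; On overlap it sends a HitBI interface message with fixed damage and short invincibility to the other actor.
; If that actor is a BP_BillieV2 with health at or below zero afterward, it creates the DeathMenu widget and shows the mouse cursor.
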(event `self.Box.OnComponentBeginOverlap`
  (params (OverlappedComponent :type "PrimitiveComponent Object Reference") (OtherActor :type "Actor Object Reference") (OtherComp :type "PrimitiveComponent Object Reference") (OtherBodyIndex :type Integer) (bFromSweep :type Boolean) (SweepResult :type "HitResult Structure (by ref)"))
  (bind _output_get (set `self.Character` OtherActor))
  (message `/Game/Blueprints/Interfaces/BPI_HitInterface.Hit_BI` _output_get 12 false false false 0 null false true false)
  (bind _asbp_billie_v2 (cast `/Game/Blueprints/Characters/BP_BillieV2` (`self.Character`)))
  (if (<= (`/Game/Blueprints/Characters/BP_BillieV2.Current_Health` _asbp_billie_v2) 0.0)
    (bind _returnvalue (`|CreateWidget` "/Game/Mods/ExampleMapMod/UI/DeathMenu.DeathMenu_C"))
    (`UserWidget.AddToViewport` _returnvalue 0)
    (set `PlayerController.bShowMouseCursor` true (`GameplayStatics.GetPlayerController` 0))))

(fn `UserConstructionScript`)