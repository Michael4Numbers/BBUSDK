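; TestEnemy is a simple test enemy Blueprint that takes hits, dies and respawns itself.
; Each hit event subtracts fixed health and plays a hit sound.
; When health runs out, it disables capsule collision, ragdolls the mesh, then after a delay spawns a fresh copy at its current transform and destroys itself.
; Its damage-check interface function always returns false.
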(event `/Game/Blueprints/Interfaces/BPI_HitInterface.Hit_BI`
  (params (DamageToDeal :type Integer) (`Slam?` :type Boolean) (`FinalHit?` :type Boolean) (`Don'tMakeInvincible?` :type Boolean) (PlayerID :type Integer) (Attacker :type "Actor Object Reference") (`MoveToSafeLocation?` :type Boolean) (`ShortInvincibility?` :type Boolean) (`Stun?` :type Boolean))
  (set `self.Health` (- (`self.Health`) 25))
  (`GameplayStatics.PlaySound2D` "/Game/Mods/ExampleMapMod/Hit.Hit" 1.0 1.0 0.0 null null)
  (if (<= (`self.Health`) 0)
    (`PrimitiveComponent.SetCollisionEnabled` (`self.CapsuleComponent`) "NoCollision")
    (`PrimitiveComponent.SetSimulatePhysics` (`self.Mesh`) true)
    (`KismetSystemLibrary.Delay` 4.0)
    (`|SpawnActorFromClass` "TestEnemy_C" (`self.GetTransform`) "Undefined" "OverrideRootScale" null null)
    (`self.K2_DestroyActor`)))

(fn `CheckCanBeDamaged_BI`
  (params (HitComponent :type "SceneComponent Object Reference"))
  (returns (`CantBeDamaged?` :type Boolean))
  (return false))

(fn `UserConstructionScript`)