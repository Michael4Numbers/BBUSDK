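; BP_BillieV2 is the Billie player character, with camera-yaw-relative movement, jumping, melee attack and health.
; A per-tick ground trace gates a launch jump; holding Jump at apex, checked through GameInstance key bindings, eases gravity scale from 1.0 to default until release.
; Attack sphere-traces forward, hitting damageable BPI_HitInterface actors with impact particles.
; Hit and heal events adjust health, with death disabling movement, though its own CheckCanBeDamaged returns false.
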(event `InputAction|Jump`
  (params (Key :type "Key Structure"))
  ;[1 1 1] Handles Jumping
  (:`Pressed`
    (if (`self.CanJump?`)
      (`self.LaunchCharacter` (0.0 0.0 1500.0) false true)
      (add `self.OnReachedJumpApex` (delegate `Event_OnApex`))))
  (:`Released`
    (if (`TimelineComponent.IsPlaying` (`self.Timeline_ScaleGravityScale`))
      (`TimelineComponent.Stop` (`self.Timeline_ScaleGravityScale`))
      (set `CharacterMovementComponent.GravityScale` (`self.Default_Gravity_Scale`) (`self.CharacterMovement`)))))

(event `Event_OnApex`
  ;[1 1 1] Handles Jumping
  (bind _iskeydown_ (`self.CheckIfKeyIsDown` "Jump")
    (:`Output`
      (if _iskeydown_
        (bind (_direction _alpha) (`Timeline|Timeline_ScaleGravityScale` :!via `PlayFromStart`)
          (:`Update`
            (set `CharacterMovementComponent.GravityScale` (`KismetMathLibrary.Lerp` 1.0 (`self.Default_Gravity_Scale`) _alpha) (`self.CharacterMovement`))))))))

(event `InputAxis|MoveForward` :overrideparent false
  (params (AxisValue :type "Float (single-precision)"))
  ;[1 1 1] Handles Player Movement based on CURRENT camera rotation
  (`self.AddMovementInput` (`KismetMathLibrary.GetForwardVector` (`KismetMathLibrary.MakeRotator` 0.0 0.0 (.yaw (`PlayerCameraManager.GetCameraRotation` (`GameplayStatics.GetPlayerCameraManager` 0))))) AxisValue))

(event `InputAxis|MoveRight` :overrideparent false
  (params (AxisValue :type "Float (single-precision)"))
  ;[1 1 1] Handles Player Movement based on CURRENT camera rotation
  (`self.AddMovementInput` (`KismetMathLibrary.GetRightVector` (`KismetMathLibrary.MakeRotator` 0.0 0.0 (.yaw (`PlayerCameraManager.GetCameraRotation` (`GameplayStatics.GetPlayerCameraManager` 0))))) AxisValue))

(event `/Game/Blueprints/Interfaces/BPI_HitInterface.Hit_BI`
  (params (DamageToDeal :type Integer) (`Slam?` :type Boolean) (`FinalHit?` :type Boolean) (`Don'tMakeInvincible?` :type Boolean) (PlayerID :type Integer) (Attacker :type "Actor Object Reference") (`MoveToSafeLocation?` :type Boolean) (`ShortInvincibility?` :type Boolean) (`Stun?` :type Boolean))
  (bind _current_health (`self.Current_Health`))
  ;[1 1 1] Damage Event
  (`KismetSystemLibrary.PrintString` (`KismetStringLibrary.Concat_StrStr` "Damaged 12.5 from " (`KismetStringLibrary.Conv_DoubleToString` (`self.Current_Health`))))
  (set `self.Current_Health` (- _current_health 12.5))
  (`KismetSystemLibrary.PrintString` (`KismetStringLibrary.Concat_StrStr` "Current Health = " (`KismetStringLibrary.Conv_DoubleToString` _current_health)))
  (if (<= (`self.Current_Health`) 0.0)
    (`KismetSystemLibrary.PrintString` "Player is Dead")
    (`CharacterMovementComponent.DisableMovement` (`self.CharacterMovement`))
    (`SkeletalMeshComponent.PlayAnimation` (`self.Mesh`) "/Game/Characters/Billie_V3/Animations/A_Billie_DeathA.A_Billie_DeathA" false)))

(event `self.ReceiveTick`
  (params (DeltaSeconds :type "Float (single-precision)"))
  (bind _capsulecomponent (`self.CapsuleComponent`))
  (bind _returnvalue (`SceneComponent.K2_GetComponentLocation` _capsulecomponent))
  ;[1 1 1] Checks if Player can jump
  (bind (_outhit _returnvalue_2) (`KismetSystemLibrary.LineTraceSingleForObjects` _returnvalue (+ _returnvalue (* (`SceneComponent.GetUpVector` _capsulecomponent) -100.0)) (`|MakeArray` "ObjectTypeQuery1" :!type "EObjectTypeQuery Enum")))
  (set `self.CanJump?` _returnvalue_2))

(event `/Game/Blueprints/Interfaces/BPI_CharMoveInterface.AddHealth_BI`
  (bind _current_health (`self.Current_Health`))
  ;[1 1 1] Add health event
  (`KismetSystemLibrary.PrintString` (`KismetStringLibrary.Concat_StrStr` "Added 12.5 to " (`KismetStringLibrary.Conv_DoubleToString` (`self.Current_Health`)) " Health."))
  (set `self.Current_Health` (+ _current_health 12.5))
  (`KismetSystemLibrary.PrintString` (`KismetStringLibrary.Concat_StrStr` "Current Health = " (`KismetStringLibrary.Conv_DoubleToString` _current_health))))

(event `InputAction|Attack`
  (params (Key :type "Key Structure"))
  (bind _returnvalue (`self.K2_GetActorLocation`))
  ;[1 1 1] Attack Event
  (:`Pressed`
    (bind (_outhits _returnvalue_2) (`KismetSystemLibrary.SphereTraceMultiForObjects` _returnvalue (+ _returnvalue (* (`self.GetActorForwardVector`) 150.0)) 0.0 (`|MakeArray` "ObjectTypeQuery1" "ObjectTypeQuery2" "ObjectTypeQuery12" "ObjectTypeQuery7" "ObjectTypeQuery3" "ObjectTypeQuery10" "ObjectTypeQuery13" "ObjectTypeQuery4" :!type "EObjectTypeQuery Enum")))
    (if _returnvalue_2
      (for _array_element _outhits
        (bind (_bblockinghit _binitialoverlap _time _distance _location _impactpoint _normal _impactnormal _physmat _hitactor _hitcomponent) (`GameplayStatics.BreakHitResult` _array_element))
        (if (`KismetSystemLibrary.DoesImplementInterface` _hitactor "/Game/Blueprints/Interfaces/BPI_HitInterface.BPI_HitInterface_C")
          (bind _cantbedamaged_ (message `/Game/Blueprints/Interfaces/BPI_HitInterface.CheckCanBeDamaged_BI` _hitactor _hitcomponent))
          (if _cantbedamaged_
            (message `/Game/Blueprints/Interfaces/BPI_HitInterface.Hit_BI` _hitactor 0 false false false 0 self false false false)
            (`GameplayStatics.SpawnEmitterAtLocation` "/Game/Particles/PS_Combat_Impact.PS_Combat_Impact" _impactpoint)))))))

(event `InputAxis|LookUp`
  (params (AxisValue :type "Float (single-precision)"))
  ;[1 1 1] Movement
  (`self.AddControllerPitchInput` AxisValue))

(event `InputAxis|LookUpRate`
  (params (AxisValue :type "Float (single-precision)"))
  ;[1 1 1] Movement
  (`self.AddControllerPitchInput` AxisValue))

(event `InputAxis|Turn`
  (params (AxisValue :type "Float (single-precision)"))
  ;[1 1 1] Movement
  (`self.AddControllerYawInput` AxisValue))

(event `InputAxis|TurnRate`
  (params (AxisValue :type "Float (single-precision)"))
  ;[1 1 1] Movement
  (`self.AddControllerYawInput` AxisValue))

(fn `CheckCanBeDamaged_BI`
  (params (HitComponent :type "SceneComponent Object Reference"))
  (returns (`CantBeDamaged?` :type Boolean))
  (return false))

(fn `Update_Health_Bar`
  (params (`Add Health?` :type Boolean)))

(fn `UserConstructionScript`)